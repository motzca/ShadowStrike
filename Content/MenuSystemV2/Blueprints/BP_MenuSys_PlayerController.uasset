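; Player controller for the menu system that drives the player character and opens the in-game pause menu.
; P (a debug stand-in for Escape) creates or reuses the pause widget, shows the cursor and pauses after a short delay.
; Tick runs focus checks on the menu's buttons while paused.
; Forward/backward axes and jump drive the cached character, while crouch, sprint, map, inventory and other actions only print placeholder text.
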(event `self.ReceiveBeginPlay`
  ;[1 1 1] At BeginPlay, get a reference to the Player Character
  (set `self.PlayerCharacterRef` (`GameplayStatics.GetPlayerCharacter` 0)))

(event `Key|Escape`
  (params (Key :type "Key Structure"))
  ;[1 1 1] Escape Key for Production Deployment only
)

(event `Key|P` :paused true
  (params (Key :type "Key Structure"))
  (bind _returnvalue (`GameplayStatics.GetPlayerController` 0))
  ;[1 1 1] Use P Key when Debugging in editor
  (:`Pressed`
    (`/Engine/EditorBlueprintResources/StandardMacros.IsValid` (`self.InGamePauseMenuRef`)
      (:`Is Valid`
        _)
      (:`Is Not Valid`
        (bind _returnvalue_2 (`|CreateWidget` "/Game/MenuSystemV2/UI/WBP_InGamePauseMenu.WBP_InGamePauseMenu_C" _returnvalue))
        (bind _output_get (set `self.InGamePauseMenuRef` _returnvalue_2))))
    (`UserWidget.AddToViewport` _output_get 0)
    (`WidgetBlueprintLibrary.SetInputMode_GameAndUIEx` _returnvalue null)
    (set `PlayerController.bShowMouseCursor` true _returnvalue)
    (`KismetSystemLibrary.Delay` 0.2)
    (`GameplayStatics.SetGamePaused` true)))

(event `self.ReceiveTick`
  (params (DeltaSeconds :type "Float (single-precision)"))
  (bind _ingamepausemenuref (`self.InGamePauseMenuRef`))
  ;[1 1 1] Event Tick for menu
  (if (`GameplayStatics.IsGamePaused`)
    (`/Engine/EditorBlueprintResources/StandardMacros.IsValid` _ingamepausemenuref
      (:`Is Valid`
        (`/Game/MenuSystemV2/UI/WBP_NavMenuButton.CheckFocus` (`/Game/MenuSystemV2/UI/WBP_InGamePauseMenu.ResumeButton` _ingamepausemenuref))
        (`/Game/MenuSystemV2/UI/WBP_NavMenuButton.CheckFocus` (`/Game/MenuSystemV2/UI/WBP_InGamePauseMenu.SettingsButton` _ingamepausemenuref))
        (`/Game/MenuSystemV2/UI/WBP_NavMenuButton.CheckFocus` (`/Game/MenuSystemV2/UI/WBP_InGamePauseMenu.QuitButton` _ingamepausemenuref))))))

(event `InputAxis|IA_MenuSys_MoveForward`
  (params (AxisValue :type "Float (single-precision)"))
  (bind _playercharacterref (`self.PlayerCharacterRef`))
  (bind (_returnvalue_roll _returnvalue_pitch _returnvalue_yaw) (`KismetMathLibrary.BreakRotator` (`Pawn.GetControlRotation` _playercharacterref)))
  ;[1 1 1] Input Axis Movement Functions
  (`Pawn.AddMovementInput` _playercharacterref (`KismetMathLibrary.GetForwardVector` (`KismetMathLibrary.MakeRotator` 0.0 0.0 _returnvalue_yaw)) AxisValue false))

(event `InputAxis|IA_MenuSys_MoveBackward`
  (params (AxisValue :type "Float (single-precision)"))
  (bind _playercharacterref (`self.PlayerCharacterRef`))
  (bind (_returnvalue_roll _returnvalue_pitch _returnvalue_yaw) (`KismetMathLibrary.BreakRotator` (`Pawn.GetControlRotation` _playercharacterref)))
  ;[1 1 1] Input Axis Movement Functions
  (`Pawn.AddMovementInput` _playercharacterref (`KismetMathLibrary.GetForwardVector` (`KismetMathLibrary.MakeRotator` 0.0 0.0 _returnvalue_yaw)) AxisValue false))

(event `InputAction|IA_MenuSys_Jump`
  (params (Key :type "Key Structure"))
  (bind _playercharacterref (`self.PlayerCharacterRef`))
  ;[1 1 1] Input Action Functions
  (:`Pressed`
    (`Character.Jump` _playercharacterref))
  (:`Released`
    (`Character.StopJumping` _playercharacterref)))

(event `InputAction|IA_MenuSys_Crouch`
  (params (Key :type "Key Structure"))
  ;[1 1 1] Input Action Functions
  (:`Pressed`
    (`KismetSystemLibrary.PrintString` "Crouch")))

(event `InputAction|IA_MenuSys_Sprint`
  (params (Key :type "Key Structure"))
  ;[1 1 1] Input Action Functions
  (:`Pressed`
    (`KismetSystemLibrary.PrintString` "Sprint")))

(event `InputAction|IA_MenuSys_EnterExit`
  (params (Key :type "Key Structure"))
  ;[1 1 1] Input Action Functions
  (:`Pressed`
    (`KismetSystemLibrary.PrintString` "Enter/Exit")))

(event `InputAction|IA_MenuSys_SpecialAbility`
  (params (Key :type "Key Structure"))
  ;[1 1 1] Input Action Functions
  (:`Pressed`
    (`KismetSystemLibrary.PrintString` "Special Ability")))

(event `InputAction|IA_MenuSys_Map`
  (params (Key :type "Key Structure"))
  ;[1 1 1] Input Action Functions
  (:`Pressed`
    (`KismetSystemLibrary.PrintString` "Map")))

(event `InputAction|IA_MenuSys_Inventory`
  (params (Key :type "Key Structure"))
  ;[1 1 1] Input Action Functions
  (:`Pressed`
    (`KismetSystemLibrary.PrintString` "Inventory")))

(event `InputAction|IA_MenuSys_Custom1`
  (params (Key :type "Key Structure"))
  ;[1 1 1] Input Action Functions
  (:`Pressed`
    (`KismetSystemLibrary.PrintString` "Custom1")))

(fn `UserConstructionScript`)